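; AI controller for guards that runs BT_Guard on BB_Guard and feeds it perception results.
; On BeginPlay it loads tuning from XML into its sight, hearing and search variables, printing the loader's error if the behavior tree fails to start.
; Perception updates write target, line of sight and last known location for sight, while other senses flag a heard noise at the stimulus location and clear line of sight.
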(event OnTargetPerceptionUpdated(AIPerception)
  (params (Actor :type Actor%20Object%20Reference) (Stimulus :type AI%20Stimulus%20Structure))
  (bind (_age _expirationage _strength _stimuluslocation _receiverlocation _tag _bsuccessfullysensed) (Utilities|Struct|BreakAIStimulus Stimulus))
  (bind _returnvalue (Class|AIPerceptionSystem|GetSenseClassforStimulus Stimulus))
  (if (== _returnvalue "/Script/AIModule.AISense_Sight")
    (if _bsuccessfullysensed
      (AI|Components|Blackboard|SetValueasObject (stale EventBeginPlay _blackboardcomponent) (Utilities|Name|MakeLiteralName "TargetActor") Actor)
      (AI|Components|Blackboard|SetValueasBool (stale EventBeginPlay _blackboardcomponent) (Utilities|Name|MakeLiteralName "HasLineOfSight") true)
      (AI|Components|Blackboard|SetValueasVector (stale EventBeginPlay _blackboardcomponent) (Utilities|Name|MakeLiteralName "LastKnownLocation") (Transformation|GetActorLocation Actor))
      (AI|Components|Blackboard|SetValueasBool (stale EventBeginPlay _blackboardcomponent) (Utilities|Name|MakeLiteralName "HeardNoise") false)
      (else
        (AI|Components|Blackboard|SetValueasBool (stale EventBeginPlay _blackboardcomponent) (Utilities|Name|MakeLiteralName "HasLineOfSight") false)))
    (else
      (AI|Components|Blackboard|SetValueasBool (stale EventBeginPlay _blackboardcomponent) (Utilities|Name|MakeLiteralName "HeardNoise") true)
      (AI|Components|Blackboard|SetValueasVector (stale EventBeginPlay _blackboardcomponent) (Utilities|Name|MakeLiteralName "LastKnownLocation") _stimuluslocation)
      (AI|Components|Blackboard|SetValueasBool (stale EventBeginPlay _blackboardcomponent) (Utilities|Name|MakeLiteralName "HasLineOfSight") false))))

(event EventTick
  (params (DeltaSeconds :type Float%20%28single-precision%29)))

(event EventBeginPlay
  (bind _blackboardcomponent (Class|AIController|UseBlackboard "/Game/AI/BB_Guard.BB_Guard"))
  (bind _returnvalue (AI|RunBehaviorTree "/Game/AI/BT_Guard.BT_Guard"))
  (bind (_outconfig _outerror) (Class|AIConfigLoaderBPLib|LoadAIConfigfromXML))
  (if _returnvalue
    (CallFunction|SetOutConfig (.sightradius _outconfig) (.losesightradius _outconfig) (.peripheralvisiondegrees _outconfig) (.hearingrange _outconfig) (.searchdurationseconds _outconfig))
    (AI|Components|Blackboard|SetValueasFloat _blackboardcomponent (Utilities|Name|MakeLiteralName "SearchTimeLeft") 0.0)
    (else
      (Development|PrintString _outerror true true "(R=1.000000,G=0.000014,B=0.002255,A=1.000000)" 3.0))))

(fn ConstructionScript)

(fn SetOutConfig
  (params (SightRadius :type Float%20%28double-precision%29) (LoseSightRadius :type Float%20%28double-precision%29) (PeripheralVisionDegrees :type Float%20%28double-precision%29) (HearingRange :type Float%20%28double-precision%29) (SearchDurationSeconds :type Float%20%28double-precision%29))
  (Variables|Default|SetSightRadius SightRadius)
  (Variables|Default|SetLoseSightRadius LoseSightRadius)
  (Variables|Default|SetPeripheralVisionDegrees PeripheralVisionDegrees)
  (Variables|Default|SetHearingRange HearingRange)
  (Variables|Default|SetSearchDurationSeconds SearchDurationSeconds))